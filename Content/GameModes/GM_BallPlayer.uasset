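; Game mode for a ball-player level that handles respawning, scoring and the win condition.
; BeginPlay creates the HUD, resets points and binds the player ball's OnDestroyed to Teleport.
; Teleport waits briefly, spawns and possesses a new ball at SpawnTransform, restores its trace and camera-arm distances, then rebinds.
; Points update the HUD; reaching six shows the win text and unlocks BP_NextLevel, while cube events only print debug text.
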(event `Respawn_actor`
  ;[1 1 1] Respawn
  (bind _asbp_player_ball_child (cast `/Game/Level_obj/Blueprint/BP_playerBall_Child` (`GameplayStatics.GetPlayerPawn` 0) :!label _label))
  (add `self.OnDestroyed` _asbp_player_ball_child (delegate `Teleport`)))

(event `self.ReceiveBeginPlay`
  ;[1 1 1] Create widget
  (bind _returnvalue (`|CreateWidget` "/Game/Level_obj/UI/BP_UserInGame.BP_UserInGame_C"))
  (bind _output_get (set `self.Current_UI` _returnvalue))
  (`UserWidget.AddToViewport` _output_get 0)
  (`self.Reset game`)
  (goto _label))

(event `Teleport` :!signature `self.OnDestroyed`
  (params (DestroyedActor :type "Actor Object Reference"))
  ;[1 1 1] Respawn
  (`KismetSystemLibrary.Delay` 0.5)
  (bind _returnvalue (`|SpawnActorFromClass` "/Game/Level_obj/Blueprint/BP_playerBall_Child.BP_playerBall_Child_C" (`KismetMathLibrary.MakeTransform` (.location (`self.Spawn_transform`)) (struct :`Yaw` -90.0) (.scale (`self.Spawn_transform`))) "Undefined" "OverrideRootScale" null null))
  (`Controller.Possess` (`GameplayStatics.GetPlayerController` 0) _returnvalue)
  (set `/Game/Level_obj/Blueprint/Parent/BP_playerBall.Trace_dist` (`self.Trace Dist`) _returnvalue)
  (set `SpringArmComponent.TargetArmLength` (`self.Target Arm Length`) (`/Game/Level_obj/Blueprint/Parent/BP_playerBall.SpringArm` _returnvalue))
  (`self.Respawn_actor`))

(event `Reset game`
  (bind _current_ui (`self.Current_UI`))
  ;[1 1 1] Reset game
  (set `self.CurrentPoints` 0)
  (set `/Game/Level_obj/UI/BP_UserInGame.points` 0 _current_ui)
  (set `/Game/Level_obj/UI/BP_UserInGame.You_win_opacit` 0.0 _current_ui))

(event `Add_points`
  ;[1 1 1] Add points
  (bind _output_get (set `self.CurrentPoints` (+ (`self.CurrentPoints`) 1)))
  (set `/Game/Level_obj/UI/BP_UserInGame.points` _output_get (`self.Current_UI`))
  (`self.end_game`))

(event `end_game`
  ;[1 1 1] End game
  (if (>= (`self.CurrentPoints`) 6)
    (set `/Game/Level_obj/UI/BP_UserInGame.You_win_opacit` 1.0 (`self.Current_UI`))
    (bind _returnvalue (`GameplayStatics.GetActorOfClass` "/Game/Level_obj/Blueprint/BP_NextLevel.BP_NextLevel_C"))
    (set `/Game/Level_obj/Blueprint/BP_NextLevel.Can_go` true _returnvalue)))

(event `Big_cube_Event`
  (`KismetSystemLibrary.PrintString` "Hello"))

(event `Normal_cube_Event`
  (`KismetSystemLibrary.PrintString` "Hello"))

(fn `UserConstructionScript`)