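; BP_playerBall is the player-controlled ball, pushed by physics impulses along camera yaw, with mouse look.
; The per-frame Jamp axis runs a line trace along the Arrow's up vector; on a hit it sets Speed, applies the vertical jump impulse and plays a sound once per contact.
; The reset to a lower Speed in the air is disconnected.
; Pause_game toggles a cached UI_MPause menu, game pause, cursor and input mode.
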(event `InputAxis|Straight`
  (params (AxisValue :type "Float (single-precision)"))
  ;[1 1 1] Player_move
  (`PrimitiveComponent.AddImpulse` (`self.Player`) (* (* AxisValue (`self.Speed`)) (`KismetMathLibrary.GetForwardVector` (`KismetMathLibrary.MakeRotator` 0.0 0.0 (.yaw (`self.GetControlRotation`))))) "None" false))

(event `InputAxis|Side`
  (params (AxisValue :type "Float (single-precision)"))
  ;[1 1 1] Player_move
  (`PrimitiveComponent.AddImpulse` (`self.Player`) (* (`KismetMathLibrary.GetRightVector` (`KismetMathLibrary.MakeRotator` 0.0 0.0 (.yaw (`self.GetControlRotation`)))) (* AxisValue (`self.Speed`))) "None" false))

(event `InputAxis|LookUD`
  (params (AxisValue :type "Float (single-precision)"))
  ;[1 1 1] Mouse
  (`self.AddControllerPitchInput` AxisValue))

(event `InputAxis|Jamp`
  (params (AxisValue :type "Float (single-precision)"))
  ;[1 1 1] Player_move
  ;;[0.5149 0.8793 1] Jamp
  (bind _returnvalue (`self.Trace`))
  (if _returnvalue
    (set `self.Speed` 2000.0)
    (`PrimitiveComponent.AddImpulse` (`self.Player`) (* (`KismetMathLibrary.MakeVector` 0.0 0.0 AxisValue) (`self.Jamp_height`)) "None" true)
    (`/Engine/EditorBlueprintResources/StandardMacros.DoOnce` false :!label _label
      (:`Completed`
        (`GameplayStatics.PlaySound2D` "/Game/Sound/Game_sound/Хлопок_1_Cue.Хлопок_1_Cue" 1.0 1.0 0.0 null null)))
    (else
      (goto _label :!via `Reset`))))

(event `InputAxis|LookLR`
  (params (AxisValue :type "Float (single-precision)"))
  ;[1 1 1] Mouse
  (`self.AddControllerYawInput` AxisValue))

(event `InputAction|Pause_game` :paused true
  (params (Key :type "Key Structure"))
  (bind _returnvalue (`GameplayStatics.GetPlayerController` 0))
  (bind _returnvalue_2 (`GameplayStatics.GetPlayerController` 0))
  (bind _pause_menu_ref (`self.Pause_menu_ref`))
  ;[1 1 1] Pause/unpause game
  (:`Pressed`
    (`/Engine/EditorBlueprintResources/StandardMacros.IsValid` (`self.Pause_menu_ref`)
      (:`Is Valid`
        _)
      (:`Is Not Valid`
        (bind _returnvalue_3 (`|CreateWidget` "/Game/Menus/UI_MPause.UI_MPause_C"))
        (set `self.Pause_menu_ref` _returnvalue_3)))
    (if (`GameplayStatics.IsGamePaused`)
      (`Widget.RemoveFromParent` _pause_menu_ref)
      (`GameplayStatics.SetGamePaused` false)
      (set `PlayerController.bShowMouseCursor` false _returnvalue)
      (`WidgetBlueprintLibrary.SetInputMode_GameOnly` _returnvalue)
      (else
        (`UserWidget.AddToViewport` _pause_menu_ref 0)
        (`GameplayStatics.SetGamePaused` true)
        (set `PlayerController.bShowMouseCursor` true _returnvalue_2)
        (`WidgetBlueprintLibrary.SetInputMode_GameAndUIEx` _returnvalue_2 _pause_menu_ref "LockInFullscreen")))))

(fn `Trace`
  (returns (ReturnValue :type Boolean))
  (bind _returnvalue (`SceneComponent.K2_GetComponentLocation` (`self.Player`)))
  (bind (_outhit _returnvalue_2) (`KismetSystemLibrary.LineTraceSingle` :`Start` _returnvalue :`End` (+ _returnvalue (* (`SceneComponent.GetUpVector` (`self.Arrow`)) (`self.Trace_dist`))) :`TraceChannel` "TraceTypeQuery2" :`DrawTime` 1.0))
  (return _returnvalue_2))

(fn `UserConstructionScript`)