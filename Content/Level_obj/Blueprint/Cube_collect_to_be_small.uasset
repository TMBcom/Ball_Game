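; Collectible cube that makes the player ball small when an actor begins overlapping it.
; The overlap runs the parent handler, then finds the player ball with GetActorOfClass and casts it to BP_playerBall_Child, without checking which actor overlapped.
; It applies the Scale value to the ball and sets fixed trace distance and spring arm length values.
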(event `self.ReceiveActorBeginOverlap`
  (params (OtherActor :type "Actor Object Reference"))
  (`parent.ReceiveActorBeginOverlap` OtherActor)
  (bind _returnvalue (`GameplayStatics.GetActorOfClass` "/Game/Level_obj/Blueprint/Parent/BP_playerBall.BP_playerBall_C"))
  (cast `/Game/Level_obj/Blueprint/BP_playerBall_Child` _returnvalue)
  (`self.SetActorScale3D` _returnvalue (`self.Scale`))
  (set `/Game/Level_obj/Blueprint/Parent/BP_playerBall.Trace_dist` 50.0 _returnvalue)
  (set `SpringArmComponent.TargetArmLength` 250.0 (`/Game/Level_obj/Blueprint/Parent/BP_playerBall.SpringArm` _returnvalue)))

(fn `UserConstructionScript`
  (`parent.UserConstructionScript`))