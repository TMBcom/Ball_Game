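; Cube_collect_to_be_big is a collectible cube that resizes the player ball when its box is overlapped, then destroys itself.
; The overlap applies configured scale, trace distance and camera arm length to BP_playerBall, and stores them with a height-raised spawn transform in GM_BallPlayer.
; BeginPlay plays a sound and binds destruction of the first cube GetActorOfClass finds, passing its cached transform to the game mode's BigCubeSpawnEvent.
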(event `self.Box1.OnComponentBeginOverlap`
  (params (OverlappedComponent :type "PrimitiveComponent Object Reference") (OtherActor :type "Actor Object Reference") (OtherComp :type "PrimitiveComponent Object Reference") (OtherBodyIndex :type Integer) (bFromSweep :type Boolean) (SweepResult :type "HitResult Structure (by ref)"))
  (bind _returnvalue (`GameplayStatics.GetActorOfClass` "/Game/Level_obj/Blueprint/Parent/BP_playerBall.BP_playerBall_C"))
  (`self.SetActorScale3D` _returnvalue (`self.Scale`))
  (set `/Game/Level_obj/Blueprint/Parent/BP_playerBall.Trace_dist` (`self.Trace Dist`) _returnvalue)
  (set `SpringArmComponent.TargetArmLength` (`self.Target Arm Length`) (`/Game/Level_obj/Blueprint/Parent/BP_playerBall.SpringArm` _returnvalue))
  (bind _asgm_ball_player (cast `/Game/GameModes/GM_BallPlayer` (`GameplayStatics.GetGameMode`)))
  (bind _spawn_transform_location (`KismetMathLibrary.BreakTransform` (`/Game/GameModes/GM_BallPlayer.Spawn_transform` _asgm_ball_player)))
  (set `/Game/GameModes/GM_BallPlayer.Spawn_transform` (`KismetMathLibrary.MakeTransform` (+ _spawn_transform_location (`KismetMathLibrary.MakeVector` 0.0 0.0 (`self.high_spawn`))) (struct) (`self.Scale`)) _asgm_ball_player)
  (bind _asgm_ball_player_2 (cast `/Game/GameModes/GM_BallPlayer` (`GameplayStatics.GetGameMode`)))
  (set `/Game/GameModes/GM_BallPlayer.Trace Dist` (`self.Trace Dist`) _asgm_ball_player_2)
  (set `/Game/GameModes/GM_BallPlayer.Target Arm Length` (`self.Target Arm Length`) _asgm_ball_player_2)
  (`self.K2_DestroyActor`))

(event `self.ReceiveBeginPlay`
  (`parent.ReceiveBeginPlay`)
  (`GameplayStatics.PlaySound2D` (`self.Sound`) 1.0 1.0 0.0 null null)
  (bind _returnvalue (`GameplayStatics.GetActorOfClass` "Cube_collect_to_be_big_C"))
  (set `self.Cube_transform` (`self.GetTransform` _returnvalue))
  (add `self.OnDestroyed` _returnvalue (delegate `Spawn_cube`)))

(event `Spawn_cube` :!signature `self.OnDestroyed`
  (params (DestroyedActor :type "Actor Object Reference"))
  (bind _asgm_ball_player (cast `/Game/GameModes/GM_BallPlayer` (`GameplayStatics.GetGameMode`)))
  (`/Game/GameModes/GM_BallPlayer.Big_cube_spawn_Event` _asgm_ball_player (`self.Cube_transform`)))

(fn `UserConstructionScript`
  (`parent.UserConstructionScript`))